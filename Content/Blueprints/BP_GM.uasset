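; Game manager that trains AI cars through generational neuroevolution, spawning batches of 50 at a PlayerStart.
; When no cars remain, it spawns the next generation from the best weights (one exact copy, the rest mutated) and restarts the killbox.
; Destruction events rank cars by distance travelled, reset each generation, until one finishes.
; Thereafter only faster completion times replace the best, each saved asynchronously to the BestAI slot.
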(event `self.ReceiveBeginPlay`
  (`KismetSystemLibrary.Delay` 1.0)
  (set `self.BestAI` (make `/Game/Blueprints/Struct_Stats` (`self.EmptyArray`) 0.0 100000.0))
  (`self.SpawnNewBatch`)
  (bind _returnvalue (`GameplayStatics.GetActorOfClass` "/Game/Blueprints/BP_Killbox.BP_Killbox_C"))
  (set `self.KILLBOX` _returnvalue))

(event `self.ReceiveTick`
  (params (DeltaSeconds :type "Float (single-precision)"))
  (if (`self.HasSpawned`)
    (bind _outactors (`GameplayStatics.GetAllActorsOfClass` "/Game/Blueprints/BP_AICar.BP_AICar_C"))
    (if (<= (`KismetArrayLibrary.Array_Length` _outactors) 0)
      (set `self.HasSpawned` false)
      (`self.SpawnNewBatch`)
      (`/Game/Blueprints/BP_Killbox.RestartKillbox` (`self.KILLBOX`)))))

(event `SpawnNewBatch`
  (bind _bestai_weights (break `/Game/Blueprints/Struct_Stats` (`self.BestAI`)))
  (bind (_bestai_weights_2 _bestai_distancetravelled _bestai_timetocomplete) (break `/Game/Blueprints/Struct_Stats` (`self.BestAI`)))
  (bind _outactors (`GameplayStatics.GetAllActorsOfClass` "/Script/Engine.PlayerStart"))
  (for _index (range 50)
    (bind (_returnvalue_location _returnvalue_rotation) (`KismetMathLibrary.BreakTransform` (`self.GetTransform` (`|GetArrayItem` _outactors))))
    (bind _returnvalue (`|SpawnActorFromClass` "/Game/Blueprints/BP_AICar.BP_AICar_C" (`KismetMathLibrary.MakeTransform` _returnvalue_location _returnvalue_rotation) "Undefined" "OverrideRootScale" null null))
    (if (== (`self.GenerationCount`) 0)
      (bind _returnvalue_2 (`AICar.GetBrain` _returnvalue))
      (`Brain.Init` _returnvalue_2 (`self.EmptyArray`) false 0.0)
      (elif (== _index 0)
        (`Brain.Init` _returnvalue_2 _bestai_weights true 0.0)
        (else
          (`Brain.Init` _returnvalue_2 _bestai_weights false 0.1)))))
  (set `self.HasSpawned` true)
  (`/Engine/EditorBlueprintResources/StandardMacros.IncrementInt` (`self.GenerationCount`)
    (:`  `
      (if (`self.HasFinished`)
        (set `self.BestAI` (make `/Game/Blueprints/Struct_Stats` _bestai_weights_2 _bestai_distancetravelled _bestai_timetocomplete))
        (else
          (set `self.BestAI` (make `/Game/Blueprints/Struct_Stats` (`self.EmptyArray`) 0.0 100000.0)))))))

(event `RegularHandleAIDestruction`
  (params (Weights :type "Array of Float (double-precision)") (DistanceTravelled :type "Float (double-precision)") (TimeToComplete :type "Float (double-precision)"))
  (bind (_bestai_weights _bestai_distancetravelled _bestai_timetocomplete) (break `/Game/Blueprints/Struct_Stats` (`self.BestAI`)))
  (if (not (`self.HasFinished`))
    (if (> DistanceTravelled _bestai_distancetravelled)
      (set `self.BestAI` (make `/Game/Blueprints/Struct_Stats` Weights DistanceTravelled _bestai_timetocomplete)))))

(event `FinishHandleAIDestruction`
  (params (Weights :type "Array of Float (double-precision)") (DistanceTravelled :type "Float (double-precision)") (TimeToComplete :type "Float (double-precision)"))
  (bind (_bestai_weights _bestai_distancetravelled _bestai_timetocomplete) (break `/Game/Blueprints/Struct_Stats` (`self.BestAI`)))
  (if (< TimeToComplete _bestai_timetocomplete)
    (set `self.BestAI` (make `/Game/Blueprints/Struct_Stats` Weights DistanceTravelled TimeToComplete))
    (set `self.HasFinished` true)
    (bind _returnvalue (`GameplayStatics.CreateSaveGameObject` "/Game/Blueprints/SaveGame_BestAI.SaveGame_BestAI_C"))
    (bind _output_get (set `self.SaveGameInstance` _returnvalue))
    (set `/Game/Blueprints/SaveGame_BestAI.BestWeights` Weights _output_get)
    (`AsyncActionHandleSaveGame.AsyncSaveGameToSlot` _output_get "BestAI")))

(fn `UserConstructionScript`)