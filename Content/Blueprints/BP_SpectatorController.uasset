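; Player controller for spectating a generation-based game, showing the current generation on screen.
; On BeginPlay it lowers resolution scale and applies one quality level to the other scalability groups via console commands, then creates the WBP_HUD widget.
; Every Tick it copies the generation count from BP_GM into the HUD text.
; The PossessSpectator event possesses a supplied pawn and clears the PossessedPawn reference.
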(event `self.ReceiveBeginPlay`
  (`self.SetQuality` "2" "50")
  (bind _returnvalue (`|CreateWidget` "/Game/Blueprints/WBP_HUD.WBP_HUD_C"))
  (bind _output_get (set `self.HUD` _returnvalue))
  (`UserWidget.AddToViewport` _output_get 0))

(event `self.ReceiveTick`
  (params (DeltaSeconds :type "Float (single-precision)"))
  (bind _asbp_gm (cast `/Game/Blueprints/BP_GM` (`GameplayStatics.GetGameMode`)))
  (`TextBlock.SetText` (`/Game/Blueprints/WBP_HUD.GenerationText` (`self.HUD`)) (`KismetTextLibrary.Conv_StringToText` (`KismetStringLibrary.Concat_StrStr` "Generation: " (`KismetStringLibrary.Conv_IntToString` (`/Game/Blueprints/BP_GM.GenerationCount` _asbp_gm))))))

(event `PossessSpectator`
  (params (Pawn :type "Pawn Object Reference"))
  (`self.Possess` self Pawn)
  (set `self.PossessedPawn` null))

(fn `SetQuality`
  (params (QualityValue :type String) (ResolutionValue :type String))
  (`KismetSystemLibrary.ExecuteConsoleCommand` (`KismetStringLibrary.Concat_StrStr` "sg.ResolutionQuality " ResolutionValue) null)
  (`KismetSystemLibrary.ExecuteConsoleCommand` (`KismetStringLibrary.Concat_StrStr` "sg.AntiAliasingQuality " QualityValue) null)
  (`KismetSystemLibrary.ExecuteConsoleCommand` (`KismetStringLibrary.Concat_StrStr` "sg.PostProcessQuality " QualityValue) null)
  (`KismetSystemLibrary.ExecuteConsoleCommand` (`KismetStringLibrary.Concat_StrStr` "sg.ShadowQuality " QualityValue) null)
  (`KismetSystemLibrary.ExecuteConsoleCommand` (`KismetStringLibrary.Concat_StrStr` "sg.GlobalIlluminationQuality " QualityValue) null)
  (`KismetSystemLibrary.ExecuteConsoleCommand` (`KismetStringLibrary.Concat_StrStr` "sg.ReflectionQuality " QualityValue) null)
  (`KismetSystemLibrary.ExecuteConsoleCommand` (`KismetStringLibrary.Concat_StrStr` "sg.TextureQuality " QualityValue) null)
  (`KismetSystemLibrary.ExecuteConsoleCommand` (`KismetStringLibrary.Concat_StrStr` "sg.EffectsQuality " QualityValue) null)
  (`KismetSystemLibrary.ExecuteConsoleCommand` (`KismetStringLibrary.Concat_StrStr` "sg.FoliageQuality " QualityValue) null)
  (`KismetSystemLibrary.ExecuteConsoleCommand` (`KismetStringLibrary.Concat_StrStr` "sg.ShadingQuality " QualityValue) null))

(fn `UserConstructionScript`)