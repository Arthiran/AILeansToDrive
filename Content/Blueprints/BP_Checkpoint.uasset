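; BP_Checkpoint is an overlap-triggered actor that switches the spectator view as the leading AI car reaches it.
; It caches the BP_Spline actor on BeginPlay, and BestCar ranks every BP_AICar by distance along that spline.
; When the overlapping car is the furthest along, the BP_SpectatorController of player 0 possesses the checkpoint's Spectator via PossessSpectator.
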(event `self.ReceiveBeginPlay`
  (bind _returnvalue (`GameplayStatics.GetActorOfClass` "/Game/Blueprints/BP_Spline.BP_Spline_C"))
  (set `self.SpineToFollow` _returnvalue))

(event `self.ReceiveActorBeginOverlap`
  (params (OtherActor :type "Actor Object Reference"))
  (bind _asbp_aicar (cast `/Game/Blueprints/BP_AICar` OtherActor))
  (bind _bestpawn (`self.BestCar`))
  (if (== _bestpawn _asbp_aicar)
    (bind _asbp_spectator_controller (cast `/Game/Blueprints/BP_SpectatorController` (`GameplayStatics.GetPlayerController` 0)))
    (`/Game/Blueprints/BP_SpectatorController.PossessSpectator` _asbp_spectator_controller (`self.Spectator`))))

(fn `BestCar`
  (returns (BestPawn :type "/Game/Blueprints/BP_AICar Object Reference"))
  (locals (BestPawnFromList :type "/Game/Blueprints/BP_AICar Object Reference") (BestDistance :type "Float (double-precision)"))
  (bind _outactors (`GameplayStatics.GetAllActorsOfClass` "/Game/Blueprints/BP_AICar.BP_AICar_C"))
  (for _array_element _outactors
    (bind _distance (`/Game/Blueprints/BP_AICar.FindDistanceAlongSpineClosestToWorldLocation` _array_element (`self.SpineToFollow`) (`self.K2_GetActorLocation` _array_element)))
    (if (>= _distance (`local.BestDistance`))
      (set `local.BestPawnFromList` _array_element)
      (set `local.BestDistance` _distance)))
  (return (`local.BestPawnFromList`)))

(fn `UserConstructionScript`)