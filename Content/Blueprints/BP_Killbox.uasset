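; BP_Killbox is a killbox actor that travels along the level's BP_Spline path; this graph handles only its movement.
; On BeginPlay it finds the spline actor and plays a timeline at a rate of 1/TimeToComplete.
; Each update maps the timeline alpha to spline distance and sets the actor's world location and rotation.
; RestartKillbox replays the timeline from the start.
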(event `self.ReceiveBeginPlay`
  (bind _returnvalue (`GameplayStatics.GetActorOfClass` "/Game/Blueprints/BP_Spline.BP_Spline_C"))
  (set `self.SplineToFollow` _returnvalue)
  (`self.MoveKillbox`))

(event `MoveKillbox`
  (bind _spline (`/Game/Blueprints/BP_Spline.Spline` (`self.SplineToFollow`)))
  (`TimelineComponent.SetPlayRate` (`self.MoveKillboxTimeline`) (/ 1.0 (`self.TimeToComplete`)))
  (bind (_direction _movetrack) (`Timeline|MoveKillboxTimeline`)
    (:`Update`
      (bind _returnvalue (`KismetMathLibrary.Lerp` 0.0 (`SplineComponent.GetSplineLength` _spline) _movetrack))
      (`self.K2_SetActorTransform` (`KismetMathLibrary.MakeTransform` (`SplineComponent.GetLocationAtDistanceAlongSpline` _spline _returnvalue "World") (`SplineComponent.GetRotationAtDistanceAlongSpline` _spline _returnvalue "World"))))))

(event `RestartKillbox`
  (`TimelineComponent.PlayFromStart` (`self.MoveKillboxTimeline`)))

(fn `UserConstructionScript`)