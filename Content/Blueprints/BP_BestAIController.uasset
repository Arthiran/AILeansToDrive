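; BP_BestAIController is a Blueprint that, despite its AI controller name, contains only graphics scalability setup and no AI logic.
; On BeginPlay it calls SetQuality with hardcoded quality and resolution strings.
; SetQuality appends those strings to scalability console variable names (sg.*) and executes each as a console command.
; The Append calls show no space between variable name and value, so the commands likely do not apply as written.
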(event `self.ReceiveBeginPlay`
  (`self.SetQuality` "5" "100"))

(fn `SetQuality`
  (params (QualityValue :type String) (ResolutionValue :type String))
  (`KismetSystemLibrary.ExecuteConsoleCommand` (`KismetStringLibrary.Concat_StrStr` "sg.ResolutionQuality " ResolutionValue) null)
  (`KismetSystemLibrary.ExecuteConsoleCommand` (`KismetStringLibrary.Concat_StrStr` "sg.AntiAliasingQuality " QualityValue) null)
  (`KismetSystemLibrary.ExecuteConsoleCommand` (`KismetStringLibrary.Concat_StrStr` "sg.PostProcessQuality " QualityValue) null)
  (`KismetSystemLibrary.ExecuteConsoleCommand` (`KismetStringLibrary.Concat_StrStr` "sg.ShadowQuality " QualityValue) null)
  (`KismetSystemLibrary.ExecuteConsoleCommand` (`KismetStringLibrary.Concat_StrStr` "sg.GlobalIlluminationQuality " QualityValue) null)
  (`KismetSystemLibrary.ExecuteConsoleCommand` (`KismetStringLibrary.Concat_StrStr` "sg.ReflectionQuality " QualityValue) null)
  (`KismetSystemLibrary.ExecuteConsoleCommand` (`KismetStringLibrary.Concat_StrStr` "sg.TextureQuality " QualityValue) null)
  (`KismetSystemLibrary.ExecuteConsoleCommand` (`KismetStringLibrary.Concat_StrStr` "sg.EffectsQuality " QualityValue) null)
  (`KismetSystemLibrary.ExecuteConsoleCommand` (`KismetStringLibrary.Concat_StrStr` "sg.FoliageQuality " QualityValue) null)
  (`KismetSystemLibrary.ExecuteConsoleCommand` (`KismetStringLibrary.Concat_StrStr` "sg.ShadingQuality " QualityValue) null))

(fn `UserConstructionScript`)